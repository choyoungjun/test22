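; Base Blueprint for a character's animation setup, holding its blend spaces, montage or sequence slots, attack combos, state-keyed animation list and input commands.
; Get/SetCharacterAnimSetup functions convert it to and from a setup table, casting between parallel enum types by integer value.
; The export fills IdleBlendDrama from AimOffset and omits AnimDramaBreak01.
; CheckAnimObject validates the animation references and logs the missing ones as an error.
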(fn CheckAnimObject
  (Variables|Default|SetLogMessage (Utilities|String|Append (Utilities|GetDisplayName self) " - "))
  (Utilities|FlowControl|Sequence
    (:then_0
      (CallFunction|ValidCheckObject (Variables|WOGR|GetMoveBlend) "[MoveBlend]")
      (CallFunction|ValidCheckObject (Variables|WOGR|GetMoveBlend_Guard) "[MoveBlendGuard]")
      (CallFunction|ValidCheckObject (Variables|WOGR|GetMoveBlend_Drama) "[MoveBlendDrama]")
      (CallFunction|ValidCheckObject (Variables|WOGR|GetIdleBlend_Drama) "[IdleBlendDrama]")
      (CallFunction|ValidCheckObject (Variables|WOGR|GetAimOffset) "[AimOffset]")
      (CallFunction|ValidCheckObject (Variables|WOGR|GetAnim_Revive) "[Anim_Revive]")
      (CallFunction|ValidCheckObject (Variables|WOGR|GetAnim_Guard) "[Anim_Guard]")
      (CallFunction|ValidCheckObject (Variables|WOGR|GetAnim_Dead_Reaction) "[Anim_Dead_Reaction]")
      (CallFunction|ValidCheckObject (Variables|WOGR|GetAnim_Break01) "[Anim_Break_01]")
      (CallFunction|ValidCheckObject (Variables|WOGR|GetAnim_Break02) "[Anim_Break_02]")
      (CallFunction|ValidCheckObject (Variables|WOGR|GetAnim_Break03) "[Anim_Break_03]")
      (CallFunction|ValidCheckObject (Variables|WOGR|GetAimUpper) "[Anim_Upper]")
      (CallFunction|ValidCheckObject (Variables|WOGR|GetAnim_TurnCast) "[Anim_TurnCast]")
      (CallFunction|ValidCheckObject (Variables|WOGR|GetAnim_DramaBreak01) "[AnimDramaBreak_01]")
      (CallFunction|ValidCheckObject (Variables|WOGR|GetAnim_AdventureRotateInPlace) "[Anim_Adventure_RotateInPlace]"))
    (:then_1
      (if (> (Utilities|Array|Length (Variables|WOGR|GetAttackComboArray)) 0)
        (CallFunction|AddLog "[AttackComboArray - ")
        (for (_array_element _array_index) (Variables|WOGR|GetAttackComboArray)
          (CallFunction|ValidCheckObject _array_element (Utilities|String|Append (Utilities|String|ToString(Integer) _array_index) ",")))
        (CallFunction|AddLog "]")))
    (:then_2
      (if (> (Utilities|Map|Length (Variables|WOGR|GetAnim%20List)) 0)
        (CallFunction|AddLog "[AnimList - ")
        (bind _keys (Utilities|Map|Keys (Variables|WOGR|GetAnim%20List)))
        (bind _values (Utilities|Map|Values (Variables|WOGR|GetAnim%20List)))
        (for (_array_element_2 _array_index_2) _values
          (CallFunction|ValidCheckObject _array_element_2 (Utilities|String|Append (Utilities|String|EnumtoString (Utilities|Array|Get(acopy) _keys _array_index_2)) ",")))
        (CallFunction|AddLog "]")))
    (:then_3
      (Class|WOGRBlueprintFunctionLibrary|LogPrint "Error" (Variables|Default|GetLogMessage)))))

(fn AddLog
  (params (B :type String))
  (Variables|Default|SetLogMessage (Utilities|String|Append (Variables|Default|GetLogMessage) B)))

(fn ValidCheckObject
  (params (InputObject :type Object%20Object%20Reference) (B :type String))
  (Utilities|IsValid InputObject
    (:Is%20Not%20Valid
      (CallFunction|AddLog B))))

(fn GetCharacterAnimSetupTable
  (return (Utilities|Struct|MakeCharacterAnimSetupTable (Utilities|GetClass self) (Variables|Default|GetComment) (Variables|WOGR|GetAnimInstance) (Variables|WOGR|GetMoveBlend) (Variables|WOGR|GetMoveBlend_Guard) (Variables|WOGR|GetMoveBlend_Drama) (Variables|WOGR|GetAimOffset) (Variables|WOGR|GetAimOffset) (Variables|WOGR|GetAttackComboArray) (CallFunction|GetInputCommand) (Variables|WOGR|GetAnim_Revive) (Variables|WOGR|GetAnim_Guard) (Variables|WOGR|GetAnim_Dead_Reaction) (Variables|WOGR|GetAnim_Break01) (Variables|WOGR|GetAnim_Break02) (Variables|WOGR|GetAnim_Break03) 0 (Variables|WOGR|GetAimUpper) (CallFunction|GetAnimList) (Variables|WOGR|GetAnim_TurnCast))))

(fn SetCharacterAnimSetup
  (params (inAnimSetupTable :type Character%20Anim%20Setup%20Table%20Structure%20%28by%20ref%29))
  (bind (_animsetupbpclass _comment _animinstance _moveblend _moveblend_guard _moveblend_drama _idleblend_drama _aimoffset _attackcomboarray _inputcommand _anim_revive _anim_guard _anim_dead_reaction _anim_break01 _anim_break02 _anim_break03 _anim_dramabreak01 _aimupper _animlist _anim_turncast) (Utilities|Struct|BreakCharacterAnimSetupTable inAnimSetupTable))
  (Utilities|FlowControl|Sequence
    (:then_0
      (Variables|WOGR|SetAnimInstance _animinstance)
      (Variables|WOGR|SetMoveBlend _moveblend)
      (Variables|WOGR|SetMoveBlend_Guard _moveblend_guard)
      (Variables|WOGR|SetMoveBlend_Drama _moveblend_drama)
      (Variables|WOGR|SetIdleBlend_Drama _idleblend_drama)
      (Variables|WOGR|SetAimOffset _aimoffset))
    (:then_1
      (Variables|WOGR|SetAttackComboArray _attackcomboarray)
      (Variables|WOGR|SetAnim_Revive _anim_revive)
      (Variables|WOGR|SetAnim_Guard _anim_guard)
      (Variables|WOGR|SetAnim_Dead_Reaction _anim_dead_reaction))
    (:then_2
      (Variables|WOGR|SetAnim_Break01 _anim_break01)
      (Variables|WOGR|SetAnim_Break02 _anim_break02)
      (Variables|WOGR|SetAnim_Break03 _anim_break03)
      (Variables|WOGR|SetAimUpper _aimupper)
      (Variables|WOGR|SetAnim_TurnCast _anim_turncast)
      (Variables|Default|SetComment _comment)
      (CallFunction|SetAnimList _animlist)
      (CallFunction|SetInputCommand _inputcommand))
    (:then_3
      (Variables|WOGR|SetAnim_DramaBreak01 _anim_dramabreak01))))

(fn GetAnimList
  (bind _keys (Utilities|Map|Keys (Variables|WOGR|GetAnim%20List)))
  (for _array_element _keys
    (Utilities|Map|Add (LocalVariables|GetLocalMap) (Utilities|Enum|ByteToEnumEInteractionAnimState (Math|Conversions|ToByte(Integer) (Math|Conversions|ToInteger(Byte) _array_element))) (.Value (Utilities|Map|Find (Variables|WOGR|GetAnim%20List) _array_element))))
  (return (LocalVariables|GetLocalMap)))

(fn SetAnimList
  (params (TableAnimList :type Map%20of%20EInteractionAnimState%20Enums%20to%20Objects :default "None"))
  (Utilities|Map|Clear (Variables|WOGR|GetAnim%20List))
  (bind _keys (Utilities|Map|Keys TableAnimList))
  (for _array_element _keys
    (Utilities|Map|Add (Variables|WOGR|GetAnim%20List) (Utilities|Enum|ByteToEnumEnumInteractionAnimState (Math|Conversions|ToByte(Integer) (Math|Conversions|ToInteger(Byte) _array_element))) (.Value (Utilities|Map|Find TableAnimList _array_element)))))

(fn GetInputCommand
  (for _array_element (Variables|WOGR|GetInputCommand)
    (Utilities|Array|Add (LocalVariables|GetLocalInputCommand) (Utilities|Struct|MakeInputCommand (.Name (Utilities|Struct|BreakStruct_InputCommand _array_element)) (Utilities|Enum|ByteToEnumEGamePadInput (Math|Conversions|ToByte(Integer) (Math|Conversions|ToInteger(Byte) (.Input (Utilities|Struct|BreakStruct_InputCommand _array_element))))) (Utilities|Enum|ByteToEnumEInputCommandState (Math|Conversions|ToByte(Integer) (Math|Conversions|ToInteger(Byte) (.inputstate (Utilities|Struct|BreakStruct_InputCommand _array_element))))) (CallFunction|GetInputCmdCondition (.SuccesCondition (Utilities|Struct|BreakStruct_InputCommand _array_element))) (CallFunction|GetInputCmdResult (.Result (Utilities|Struct|BreakStruct_InputCommand _array_element))))))
  (return (LocalVariables|GetLocalInputCommand)))

(fn SetInputCommand
  (params (NewParam :type Array%20of%20Input%20Command%20Structures))
  (Utilities|Array|Clear (Variables|WOGR|GetInputCommand))
  (for _array_element NewParam
    (Utilities|Array|Add (Variables|WOGR|GetInputCommand) (Utilities|Struct|MakeStruct_InputCommand (.Name (Utilities|Struct|BreakInputCommand _array_element)) (Utilities|Enum|ByteToEnumEnumGamePadInput (Math|Conversions|ToByte(Integer) (Math|Conversions|ToInteger(Byte) (.Input (Utilities|Struct|BreakInputCommand _array_element))))) (Utilities|Enum|ByteToEnumEnumInputCommandState (Math|Conversions|ToByte(Integer) (Math|Conversions|ToInteger(Byte) (.inputstate (Utilities|Struct|BreakInputCommand _array_element))))) (CallFunction|GetInputCmdCondition2 (.SuccesCondition (Utilities|Struct|BreakInputCommand _array_element))) (CallFunction|GetInputCmdResult2 (.Result (Utilities|Struct|BreakInputCommand _array_element)))))))

(fn GetInputCmdCondition
  (params (NewParam :type Array%20of%20Struct%20Input%20Command%20Condition%20Structures))
  (for _array_element NewParam
    (Utilities|Array|Add (LocalVariables|GetNewLocalVar_0) (Utilities|Struct|MakeInputCommandCondition (Utilities|Enum|ByteToEnumEInteractionAnimState (Math|Conversions|ToByte(Integer) (Math|Conversions|ToInteger(Byte) (.animstate _array_element)))) (.section _array_element) (.cmd _array_element))))
  (return (LocalVariables|GetNewLocalVar_0)))

(fn GetInputCmdResult
  (params (NewParam :type Array%20of%20Struct%20Input%20Command%20Result%20Structures))
  (for _array_element NewParam
    (Utilities|Array|Add (LocalVariables|GetNewLocalVar_0) (Utilities|Struct|MakeInputCommandResult (Utilities|Enum|ByteToEnumEInteractionAnimState (Math|Conversions|ToByte(Integer) (Math|Conversions|ToInteger(Byte) (.animstate _array_element)))) (.section _array_element) (.delay _array_element) (.cmd _array_element))))
  (return (LocalVariables|GetNewLocalVar_0)))

(fn GetInputCmdCondition2
  (params (NewParam :type Array%20of%20Input%20Command%20Condition%20Structures))
  (for _array_element NewParam
    (Utilities|Array|Add (LocalVariables|GetNewLocalVar_0) (Utilities|Struct|MakeStruct_InputCommandCondition (Utilities|Enum|ByteToEnumEnumInteractionAnimState (Math|Conversions|ToByte(Integer) (Math|Conversions|ToInteger(Byte) (.animstate _array_element)))) (.section _array_element) (.cmd _array_element))))
  (return (LocalVariables|GetNewLocalVar_0)))

(fn GetInputCmdResult2
  (params (NewParam :type Array%20of%20Input%20Command%20Result%20Structures))
  (for _array_element NewParam
    (Utilities|Array|Add (LocalVariables|GetNewLocalVar_0) (Utilities|Struct|MakeStruct_InputCommandResult (Utilities|Enum|ByteToEnumEnumInteractionAnimState (Math|Conversions|ToByte(Integer) (Math|Conversions|ToInteger(Byte) (.animstate _array_element)))) (.section _array_element) (.delay _array_element) (.cmd _array_element))))
  (return (LocalVariables|GetNewLocalVar_0)))