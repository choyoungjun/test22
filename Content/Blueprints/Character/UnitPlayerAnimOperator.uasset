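; UnitPlayerAnimOperator is a player-unit animation operator meant to turn input-state actions into montages, but it is largely disconnected.
; ActionMontage calls PlayMontage, which only creates a dynamic montage, using the section name as slot name.
; PlayInputstatePressAction's condition matching, AnimState lookup and command dispatch are unwired, leaving it without effect.
; IsPlayMontage always returns true, and ChangeAction, BeginPlay and Tick are empty.
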(event Custom|ActionMontage
  (params (AnimMontage :type Anim%20Montage%20Object%20Reference) (StartSectionName :type Name) (AnimState :type EnumInteractionAnimState%20Enum :default "NewEnumerator20"))
  (CallFunction|PlayMontage AnimMontage StartSectionName 0.0 AnimState))

(event EventBeginPlay)

(event EventTick
  (params (DeltaSeconds :type Float%20%28single-precision%29)))

(fn ChangeAction)

(fn IsPlayMontage
  (return true))

(fn PlayMontage
  (params (AnimMontage :type Anim%20Montage%20Object%20Reference) (StartSectionName :type Name) (DelayTime :type Float%20%28double-precision%29) (AnimState :type EnumInteractionAnimState%20Enum :default "NewEnumerator20"))
  (Class|AnimMontage|CreateSlotAnimationasDynamicMontagewithBlendSettings AnimMontage StartSectionName (Utilities|Struct|MakeMontageBlendSettings 0 "(CustomCurve=None,BlendTime=0.200000,BlendOption=Linear)" "Standard") (Utilities|Struct|MakeMontageBlendSettings 0 "(CustomCurve=None,BlendTime=0.200000,BlendOption=Linear)" "Standard") 1.0 1 -1.0))

(fn PlayInputstatePressAction
  (params (InputPin :type Array%20of%20Struct%20Input%20Command%20Condition%20Structures) (InputPin2 :type Array%20of%20Struct%20Input%20Command%20Result%20Structures))
  (if (Utilities|Array|IsValidIndex InputPin)
    (bind (_array_element _array_index) (Utilities|Array|ForEachLoopwithBreak InputPin)
      (:Completed
        (return)))
    (elif (not (Utilities|Array|IsValidIndex InputPin2)) ; Command Condition  가 없는경우는 그냥 0번째 Result실행
      (return))))