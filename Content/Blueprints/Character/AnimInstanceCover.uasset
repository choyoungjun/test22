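; AnimInstanceCover declares a common, interface-style API for driving character animation instances, with every function left as an empty stub or default return.
; Gameplay calls cover montages, movement, guard, damage, death, revive and turn casting, plus queries for combo, command and animation lists.
; Presentation calls cover aim and rotation, parent mesh, eye blink, lip sync, drama idle and move blend spaces, and ship flag rotation.
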(fn PlayEventMontage
  (params (Montage%20to%20Play :type Anim%20Montage%20Object%20Reference) (StopAllMontages :type Boolean))
  (return 0.0))

(fn SetAimRotation
  (params (Rotation :type Vector%202D%20Structure)))

(fn SetAimRotationAlpha
  (params (Rotation :type Vector%202D%20Structure) (NewAlpha :type Float%20%28single-precision%29)))

(fn IsAnyAnimMontagePlaying
  (return false))

(fn AttackComboList
  (return 0))

(fn InputCommandList
  (return 0))

(fn AnimationList
  (return "NewEnumerator20"))

(fn ResetParentMesh
  (return false))

(fn BreakAnimation)

(fn ReviveAnimation)

(fn MoveAnimation)

(fn DamageAnimation
  (params (DamageAnimation :type EnumDamageAnimation%20Enum :default "NewEnumerator0")))

(fn DeathAnimation)

(fn CurrentAnimInstance
  (return 0))

(fn GuardAnimation)

(fn AnimNotifyGuardEnd)

(fn UnitGuardProperty
  (return false))

(fn PlayActionDramaAnimation
  (params (Montage :type Anim%20Montage%20Object%20Reference) (StartTime :type Float%20%28single-precision%29) (PlayTime :type Float%20%28single-precision%29) (StopAllMontage :type Boolean)))

(fn GetCurrentProperty
  (return 0))

(fn SetParentMesh
  (params (NewMesh :type Skeletal%20Mesh%20Component%20Object%20Reference))
  (return 0))

(fn InitializeInstance
  (params (CharacterSetup :type Character%20Anim%20Setup%20Bp%20Base%20Object%20Reference)))

(fn TurnCastAnimation
  (params (IsTurnCast :type Boolean) (Animation :type Anim%20Sequence%20Object%20Reference)))

(fn SequenceAnimation
  (params (anim :type Anim%20Sequence%20Object%20Reference)))

(fn UpdateRotationAnimation)

(fn EndRotationAnimation)

(fn SetAimUpperRotationAlpha
  (params (Rotation :type Vector%202D%20Structure) (NewAlpha :type Float%20%28single-precision%29)))

(fn SetEnableEyeBlink
  (params (EnableEyeBlink :type Boolean)))

(fn PlayLipSync
  (params (FacialLipSyncType :type EnumFacialLipSyncType%20Enum :default "NewEnumerator0")))

(fn StopLipSync)

(fn PlayAnimDramaIdle)

(fn StopAnimation)

(fn GuardEndAnimation)

(fn SetShipFlagRotation
  (params (FlagRotation :type Rotator)))

(fn ChangeDramaIdleBlendSpace
  (params (BlendSpace :type Blend%20Space%20Base%20Object%20Reference)))

(fn ChangeDramaMoveBlendSpace
  (params (BlendSpace :type Blend%20Space%20Base%20Object%20Reference)))

(fn GetDeadReactionAnimation
  (return 0))